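; BP_Forthwall is a wall actor that slides along with the player and nudges them away on contact.
; Each tick it matches its root's world X to player pawn 0 while keeping its own Y and Z.
; When a BP_Player begins overlapping it, the wall teleports that player a small fixed offset along positive Y, printing debug strings for each overlap.
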(event EventBeginPlay)

(event Collision|EventActorBeginOverlap
  (params (OtherActor :type Actor%20Object%20Reference))
  (Development|PrintString "OVERLAP")
  (bind _asbp_player (Utilities|Casting|CastToBP_Player OtherActor)
    (:then
      (Development|PrintString "is a player")
      (Class|Actor|AddActorWorldTransform _asbp_player (Math|Transform|MakeTransform (Math|Vector|MakeVector 0.0 1e+01 0.0) "0, 0, 0" "1,1,1") false true))
    (:CastFailed
      (Development|PrintString "aint a player"))))

(event EventTick
  (params (DeltaSeconds :type Float%20%28single-precision%29))
  (bind _defaultsceneroot (Variables|Default|GetDefaultSceneRoot))
  (bind _returnvalue (Transformation|GetWorldLocation _defaultsceneroot))
  (Transformation|SetWorldLocation (Variables|Default|GetDefaultSceneRoot) (Math|Vector|MakeVector (.x (Transformation|GetWorldLocation (Variables|/Script/Engine.Actor|GetRootComponent (Game|Player|GetPlayerPawn 0)))) (.y _returnvalue) (.z _returnvalue)) false false))

(fn ConstructionScript)