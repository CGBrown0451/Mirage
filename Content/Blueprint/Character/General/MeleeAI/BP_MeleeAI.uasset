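; BP_MeleeAI is the AI controller for melee characters, supplying player-relative movement targets to the BP_MeleeAITree behavior tree.
; On possess it runs the tree and stores the player character in the Blackboard.
; Tick accumulates a timer and, past the change interval, flips DesiredDirection and sets DesiredLocation to one side of the player along world X.
; The timer is never reset here, so flipping repeats every tick thereafter; DecideDirection is empty.
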(event Custom|Decide%20Direction)

(event EventBeginPlay)

(event EventTick
  (params (DeltaSeconds :type Float%20%28single-precision%29))
  (bind _returnvalue (Utilities|Name|MakeLiteralName "DesiredLocation"))
  (bind _returnvalue_2 (AI|GetBlackboard 0))
  (bind _returnvalue_3 (Utilities|Name|MakeLiteralName "DesiredDirection"))
  (bind _output_get (Variables|Default|SetDesiredDirectionTimer (+ (Variables|Default|GetDesiredDirectionTimer) DeltaSeconds)))
  (if (> _output_get (Variables|Default|GetDesiredDirectionChangeTime))
    (AI|Components|Blackboard|SetValueasBool _returnvalue_2 _returnvalue_3 (not (ScalableFloat|GetValueasBool _returnvalue_2 _returnvalue_3)))
    (bind _asbp_base_character (Utilities|Casting|CastToBP_BaseCharacter (AI|Components|Blackboard|GetValueasObject _returnvalue_2 (Utilities|Name|MakeLiteralName "Player"))))
    (if (ScalableFloat|GetValueasBool _returnvalue_2 _returnvalue_3)
      (AI|Components|Blackboard|SetValueasVector _returnvalue_2 _returnvalue (Math|Vector|MakeVector (+ (.X (Math|Vector|BreakVector (Transformation|GetActorLocation _asbp_base_character))) 6e+01) (.Y (Math|Vector|BreakVector (Transformation|GetActorLocation _asbp_base_character))) (.Z (Math|Vector|BreakVector (Transformation|GetActorLocation _asbp_base_character)))))
      (else
        (AI|Components|Blackboard|SetValueasVector _returnvalue_2 _returnvalue (Math|Vector|MakeVector (- (.X (Math|Vector|BreakVector (Transformation|GetActorLocation _asbp_base_character))) 6e+01) (.Y (Math|Vector|BreakVector (Transformation|GetActorLocation _asbp_base_character))) (.Z (Math|Vector|BreakVector (Transformation|GetActorLocation _asbp_base_character)))))))))

(event EventPossess
  (params (PossessedPawn :type Pawn%20Object%20Reference))
  (AI|RunBehaviorTree "/Game/Blueprint/Character/General/MeleeAI/BP_MeleeAITree.BP_MeleeAITree")
  (AI|Components|Blackboard|SetValueasObject (Variables|Default|GetBlackboard) (Utilities|Name|MakeLiteralName "Player") (Game|GetPlayerCharacter 0)))

(fn ConstructionScript)