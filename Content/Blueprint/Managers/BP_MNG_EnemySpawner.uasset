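; Enemy spawner manager Blueprint that spawns a wave of basic enemies, labeled as wave 3 in its debug print.
; The wave function spawns two BP_EnemyBasic actors at the Forewall box with random Y offsets, passing the player pawn and spawn health, then sets the enemy count.
; A separate Fill array helper stores a target's world X position in the trigger bar locations array at a given index.
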(fn ConstructionScript)

(fn NewFunction0
  (bind _returnvalue (Math|Random|RandomFloat))
  (bind _forewall (Variables|Default|Getforewall))
  (bind _returnvalue_2 (* _returnvalue 1e+01))
  (bind _box (Variables|/Game/Blueprint/Walls/BP_Forewall.BP_Forewall_C|GetBox _forewall))
  (bind _returnvalue_3 (Transformation|GetWorldLocation _box))
  (bind _returnvalue_4 (+ (.y _returnvalue_3) _returnvalue_2))
  (Development|PrintString "Wave 3 - spawns 2 enemy")
  (bind _asbp_player (Utilities|Casting|CastToBP_Player (Game|Player|GetPlayerPawn 0)))
  (Game|SpawnActorfromClass "/Game/Blueprint/Character/enemy/BP_EnemyBasic.BP_EnemyBasic_C" (Math|Transform|MakeTransform (Math|Vector|MakeVector (.x _returnvalue_3) _returnvalue_4 (.z _returnvalue_3)) "0, 0, 0" "1,1,1") "Undefined" 0 _asbp_player 2.0 0)
  (Game|SpawnActorfromClass "/Game/Blueprint/Character/enemy/BP_EnemyBasic.BP_EnemyBasic_C" (Math|Transform|MakeTransform (Math|Vector|MakeVector (.x _returnvalue_3) _returnvalue_4 (.z _returnvalue_3)) "0, 0, 0" "1,1,1") "Undefined" 0 _asbp_player 2.0 0)
  (Variables|Default|SetEnemy%20count 2))