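; BP_Backwall is a wall actor that repositions itself along the X axis relative to the first player's pawn.
; On Tick it adds its root's world X to the pawn's and, when that sum exceeds a fixed threshold, moves itself to a fixed X offset from the pawn, keeping Y and Z.
; The check uses the sum of the two positions, not the distance between them.
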(event EventBeginPlay)

(event Collision|EventActorBeginOverlap
  (params (OtherActor :type Actor%20Object%20Reference)))

(event EventTick
  (params (DeltaSeconds :type Float%20%28single-precision%29))
  (bind _returnvalue (Game|Player|GetPlayerPawn 0))
  (bind _defaultsceneroot (Variables|Default|GetDefaultSceneRoot))
  (bind _returnvalue_2 (Transformation|GetWorldLocation _defaultsceneroot))
  (bind _rootcomponent (Variables|/Script/Engine.Actor|GetRootComponent _returnvalue))
  (bind _returnvalue_3 (Transformation|GetWorldLocation _rootcomponent))
  (if (> (+ (.x (Transformation|GetWorldLocation (Variables|Default|GetDefaultSceneRoot))) (.x _returnvalue_3)) 2e+03)
    (Transformation|SetWorldLocation (Variables|Default|GetDefaultSceneRoot) (Math|Vector|MakeVector (+ (.x _returnvalue_3) 2e+03) (.y _returnvalue_2) (.z _returnvalue_2)) false false)))

(fn ConstructionScript)