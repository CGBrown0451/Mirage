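; Base character Blueprint that turns inputs buffered on BP_CharacterController into punching, crouching and left/right facing.
; Tick treats a running lock timer or falling as locked, which clears any buffered hit.
; When unlocked, it applies hit and crouch, disables PunchBox collision, then rotates the capsule to face Direction.
; A hit starts a short lock and enables PunchBox collision, which that same Tick sequence switches off again.
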(event Custom|DoHit
  (Collision|SetCollisionEnabled (Variables|Default|GetPunchBox) "QueryOnly")
  (Variables|Default|SetLockTime 0.5))

(event Custom|DoCrouch
  (if (not (AI|Components|NavMovement|IsCrouching (Variables|Character|GetCharacterMovement)))
    (Character|Crouch)))

(event Custom|DoUncrouch
  (Character|UnCrouch))

(event Custom|DoJump
  (Character|Jump))

(event EventBeginPlay
  (bind _asbp_character_controller (Utilities|Casting|CastToBP_CharacterController (Pawn|GetController)))
  (Variables|Default|SetControl _asbp_character_controller)
  (Variables|Default|SetbUseControllerRotationYaw false))

(event Collision|EventActorBeginOverlap
  (params (OtherActor :type Actor%20Object%20Reference)))

(event EventTick
  (params (DeltaSeconds :type Float%20%28single-precision%29))
  (bind _capsulecomponent (Variables|Collision|GetCapsuleComponent))
  (bind _control (Variables|Default|GetControl))
  (bind _control_2 (Variables|Default|GetControl))
  (bind _direction (Variables|/Game/Blueprint/Character/General/BP_CharacterController.BP_CharacterController_C|Getdirection _control_2))
  (if (> (Variables|Default|GetLockTime) 0.0)
    (Variables|Default|SetLockTime (- (Variables|Default|GetLockTime) DeltaSeconds))
    (Variables|Default|SetisLocked true :!label _label)
    (Variables|/Game/Blueprint/Character/General/BP_CharacterController.BP_CharacterController_C|SethitBuffered _control false)
    (elif (AI|Components|NavMovement|IsFalling (Variables|Character|GetCharacterMovement))
      (goto _label)
      (else
        (Variables|Default|SetisLocked false)
        (Utilities|FlowControl|Sequence
          (:then_0
            (if (Variables|/Game/Blueprint/Character/General/BP_CharacterController.BP_CharacterController_C|GethitBuffered _control)
              (CallFunction|DoHit)))
          (:then_1
            (if (Variables|/Game/Blueprint/Character/General/BP_CharacterController.BP_CharacterController_C|GetcrouchBuffered _control)
              (CallFunction|DoCrouch)
              (else
                (CallFunction|DoUncrouch))))
          (:then_2
            (Collision|SetCollisionEnabled (Variables|Default|GetPunchBox) "NoCollision")
            (Development|PrintString (Utilities|String|ToString(Integer) _direction))
            (if (== _direction -1)
              (Transformation|SetWorldRotation _capsulecomponent "0,-180.000000,0.000000" false false)
              (elif (== _direction 1)
                (Transformation|SetWorldRotation _capsulecomponent "0, 0, 0" false false)))))))))

(fn ConstructionScript)