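; Game mode that starts a low, pitched-down ambient rumble and sets up the on-screen text manager at BeginPlay.
; Creates a BP_TextManger widget targeting the player character and adds it to the viewport.
; Scans actors implementing the BP_Walllocator interface, skips the forewall, and hands the widget reference to each BP_Triggerbar, with debug prints along the way.
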(event EventBeginPlay
  (Audio|PlaySound2D "/Game/Sounds/Cool__meloncholy_rumble__bass.Cool__meloncholy_rumble__bass" 0.2 0.5 0.0 0 0)
  (bind _asbp_player (Utilities|Casting|CastToBP_Player (Game|GetPlayerCharacter 0)))
  (bind _returnvalue (UserInterface|CreateWidget "/Game/Blueprint/Managers/BP_TextManger.BP_TextManger_C" (Game|GetPlayerController 0) _asbp_player))
  (bind _output_get (Variables|Default|SetTextManager _returnvalue))
  (UserInterface|Viewport|AddtoViewport _output_get 0)
  (Widget|SetVisibility _output_get "Visible")
  (bind _outactors (Actor|GetAllActorswithInterface "/Game/Blueprint/Managers/BP_Walllocator.BP_Walllocator_C"))
  (for (_array_element _array_index) _outactors
    (Development|PrintString (Utilities|String|ToString(Integer) _array_index))
    (if (== _array_element "/Game/Blueprint/Walls/BP_Forewall.BP_Forewall")
      (Development|PrintString "forewall - ignoring")
      (else
        (Development|PrintString "triggerwall")
        (bind _asbp_triggerbar (Utilities|Casting|CastToBP_Triggerbar _array_element))
        (Variables|/Game/Blueprint/Walls/BP_Triggerbar.BP_Triggerbar_C|Setclassref _asbp_triggerbar (Variables|Default|GetTextManager)))))
  (Development|PrintString "scan complete"))

(fn ConstructionScript)