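; BP_playerdummy is a dummy character in the enemy folder that removes itself when its health runs out.
; On BeginPlay it sets HitDamage and initializes Health from SpawnHealth.
; It polls Health every Tick after calling the parent Tick, then prints a debug string and destroys the actor once Health reaches zero or below.
; The graph itself contains no damage-handling logic.
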(event EventBeginPlay
  (Variables|Default|SetHitDamage 1.0)
  (Variables|Default|SetHealth (Variables|Default|GetSpawnHealth)))

(event EventTick
  (params (DeltaSeconds :type Float%20%28single-precision%29))
  (|CallParentFunction DeltaSeconds)
  (if (<= (Variables|Default|GetHealth) 0.0)
    (Development|PrintString "killing self")
    (Actor|DestroyActor)))

(fn ConstructionScript
  (|CallParentFunction))