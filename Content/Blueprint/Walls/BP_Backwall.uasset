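; BP_Backwall is a wall actor that trails the player pawn along the world X axis.
; Each Tick it compares its root's X with player 0's and, when more than 2000 units ahead on +X, snaps to exactly that distance.
; The wall only ever moves toward -X, so it never retreats when the player turns back, and its Y and Z stay unchanged.
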(event EventBeginPlay)

(event EventTick
  (params (DeltaSeconds :type Float%20%28single-precision%29))
  (bind _returnvalue (Game|Player|GetPlayerPawn 0))
  (bind _defaultsceneroot (Variables|Default|GetDefaultSceneRoot))
  (bind _defaultsceneroot_2 (Variables|Default|GetDefaultSceneRoot))
  (bind _returnvalue_2 (Transformation|GetWorldLocation _defaultsceneroot))
  (bind _returnvalue_3 (Transformation|GetWorldLocation _defaultsceneroot_2))
  (bind _rootcomponent (Variables|/Script/Engine.Actor|GetRootComponent _returnvalue))
  (bind _returnvalue_4 (Transformation|GetWorldLocation _rootcomponent))
  (bind _returnvalue_5 (- (.x _returnvalue_3) (.x _returnvalue_4)))
  (if (> _returnvalue_5 2e+03)
    (Transformation|SetWorldLocation (Variables|Default|GetDefaultSceneRoot) (Math|Vector|MakeVector (- (.x _returnvalue_3) (- _returnvalue_5 2e+03)) (.y _returnvalue_2) (.z _returnvalue_2)) false false)))

(fn ConstructionScript)