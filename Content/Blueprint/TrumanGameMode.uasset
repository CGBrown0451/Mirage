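; TrumanGameMode is a game mode that creates the BP_TextManger widget, passes itself to it and shows it on the viewport.
; Tick calls TextFires with zero every frame and enters a self-looping two-second Delay that increments Testvar, passes it to TextFires and prints it as debug output.
; A TextVisable branch for toggling widget visibility is left unconnected.
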(event EventBeginPlay
  (bind _returnvalue (UserInterface|CreateWidget "/Game/Blueprint/BP_TextManger.BP_TextManger_C" (Game|GetPlayerController 0) self))
  (bind _output_get (Variables|Default|SetTextManager _returnvalue))
  (UserInterface|Viewport|AddtoViewport _output_get 0)
  (Widget|SetVisibility _output_get "Visible"))

(event EventTick
  (params (DeltaSeconds :type Float%20%28single-precision%29))
  (bind _asbp_text_manger (Utilities|Casting|CastToBP_TextManger (Variables|Default|GetTextManager)))
  (Default|TextFires _asbp_text_manger)
  (Utilities|FlowControl|Delay 2.0 :!label _label)
  (bind _output_get (Variables|Default|Settestvar (+ (Variables|Default|Gettestvar) 1)))
  (Default|TextFires _asbp_text_manger _output_get)
  (Development|PrintString (Utilities|String|ToString(Integer) _output_get))
  (goto _label))

(fn ConstructionScript)