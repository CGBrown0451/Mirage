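; BP_Dummy is a dummy character that attacks on a timer and reacts to being hit.
; Tick counts down HitCountDown, then resets it to HitTime and calls DoHit.
; GetHit prints the damage and struck component, then calls LaunchCharacter with scaled backward and up vectors multiplied together rather than added.
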(event EventBeginPlay
  (|CallParentFunction) ; This node is disabled and will not be called.\nDrag off pins to build functionality.
)

(event Collision|EventActorBeginOverlap
  (params (OtherActor :type Actor%20Object%20Reference)))

(event EventTick
  (params (DeltaSeconds :type Float%20%28single-precision%29))
  (|CallParentFunction DeltaSeconds)
  (bind _output_get (Variables|Default|SetHitCountDown (- (Variables|Default|GetHitCountDown) DeltaSeconds)))
  (if (< _output_get 0.0)
    (Variables|Default|SetHitCountDown (Variables|Default|GetHitTime))
    (CallFunction|DoHit)))

(event EventGetHit
  (params (Damage :type Float%20%28single-precision%29) (ComponentHit :type Actor%20Component%20Object%20Reference))
  (bind _capsulecomponent (Variables|Default|GetCapsuleComponent))
  (Development|PrintString (Utilities|String|Append "OW " (Utilities|String|ToString(Float) Damage) (Utilities|GetDisplayName ComponentHit)))
  (Character|LaunchCharacter (* (* (* (Math|Vector|GetForwardVector _capsulecomponent) -1) 6e+04) (* (Math|Vector|GetUpVector _capsulecomponent) 6e+05)) false false))

(fn ConstructionScript
  (|CallParentFunction))