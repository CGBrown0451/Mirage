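; Character controller that turns player input into movement and buffered actions for the player's BP_BaseCharacter pawn, cached on BeginPlay.
; Axis inputs are rounded into X and Y movement vectors while the character is unlocked, with horizontal input also stored as Direction.
; Crouch is buffered while held and Hit latches on press without being cleared.
; Tick checks both buffers against the lock state, but those branches are still empty.
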(event Custom|GetPlayer
  (bind _asbp_base_character (Utilities|Casting|CastToBP_BaseCharacter (Game|Player|GetPlayerPawn 0)))
  (Variables|Default|Setcontrolled _asbp_base_character))

(event EventBeginPlay
  (CallFunction|GetPlayer))

(event EventTick
  (params (DeltaSeconds :type Float%20%28single-precision%29))
  (bind _controlled (Variables|Default|Getcontrolled))
  (bind _islocked (Variables|/Game/Blueprint/Character/General/BP_BaseCharacter.BP_BaseCharacter_C|GetisLocked _controlled))
  (Utilities|FlowControl|Sequence
    (:then_0
      (if (Variables|Default|GethitBuffered)
        (if _islocked
          _)))
    (:then_1
      (if _islocked
        (if (Variables|Default|GetcrouchBuffered)
          _)))))

(event Input|ActionEvents|InputActionCrouch
  (params (Key :type Key%20Structure :default "None"))
  (:Pressed
    (Variables|Default|SetcrouchBuffered true))
  (:Released
    (Variables|Default|SetcrouchBuffered false)))

(event Input|ActionEvents|InputActionHit
  (params (Key :type Key%20Structure :default "None"))
  (:Pressed
    (Variables|Default|SethitBuffered true)))

(event Input|ActionEvents|InputActionJump
  (params (Key :type Key%20Structure :default "None")))

(event Input|AxisEvents|InputAxisLeft/Right
  (params (AxisValue :type Float%20%28single-precision%29))
  (bind _returnvalue (Math|Float|Round AxisValue))
  (if (not (Variables|/Game/Blueprint/Character/General/BP_BaseCharacter.BP_BaseCharacter_C|GetisLocked (Variables|Default|Getcontrolled)))
    (Class|PawnMovementComponent|AddInputVector (Variables|/Script/Engine.Character|GetCharacterMovement (Variables|Default|Getcontrolled)) (Math|Vector|MakeVector (Math|Conversions|ToFloat(Integer) _returnvalue) 0.0 0.0) false)
    (Variables|Default|Setdirection _returnvalue)))

(event Input|AxisEvents|InputAxisUp/Down
  (params (AxisValue :type Float%20%28single-precision%29))
  (if (not (Variables|/Game/Blueprint/Character/General/BP_BaseCharacter.BP_BaseCharacter_C|GetisLocked (Variables|Default|Getcontrolled)))
    (Class|PawnMovementComponent|AddInputVector (Variables|/Script/Engine.Character|GetCharacterMovement (Variables|Default|Getcontrolled)) (Math|Vector|MakeVector 0.0 (Math|Conversions|ToFloat(Integer) (Math|Float|Round AxisValue)) 0.0) false)))

(fn ConstructionScript)