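; BP_Triggerbar is a one-shot story trigger that fires narration and text as the player passes it.
; Tick compares the player's X to the Box's rather than using overlaps, then plays the voice line chosen by TextToFire and calls BP_TextManger.
; Regular bars then destroy themselves.
; Index 6 runs the ending: it marks the player hopeless, aligns the light beam, sets EndGame, shows text and opens NewMap.
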(event Custom|fire%20sound
  (bind _voice_volume (Variables|Default|GetVoice%20volume))
  (switch int (Variables|Default|GetText%20to%20fire)
    (:0
      (Audio|PlaySound2D "/Game/Sounds/allthings.allthings" _voice_volume 1.0 0.0 0 0 :!label _label))
    (:1
      (Audio|PlaySound2D "/Game/Sounds/lostsoulcrush.lostsoulcrush" _voice_volume 1.0 0.0 0 0))
    (:2
      (Audio|PlaySound2D "/Game/Sounds/keepfight.keepfight" _voice_volume 1.0 0.0 0 0))
    (:3
      (Audio|PlaySound2D "/Game/Sounds/hope_burns.hope_burns" _voice_volume 1.0 0.0 0 0))
    (:4
      (Audio|PlaySound2D "/Game/Sounds/reignite.reignite" _voice_volume 1.0 0.0 0 0))
    (:5
      (goto _label))))

(event EventBeginPlay)

(event Collision|EventActorBeginOverlap
  (params (OtherActor :type Actor%20Object%20Reference)))

(event EventTick
  (params (DeltaSeconds :type Float%20%28single-precision%29))
  (bind _light_beam (Variables|Default|Getlight%20beam))
  (bind _world (Variables|/Game/Blueprint/Eviros/bp_Beam_End.bp_Beam_End_C|Getworld _light_beam))
  (bind _returnvalue (Transformation|GetWorldLocation _world))
  (if (not (Variables|Default|GetHas%20been%20tripped?))
    (if (<= (.x (Transformation|GetWorldLocation (Variables|/Script/Engine.Actor|GetRootComponent (Game|Player|GetPlayerPawn 0)))) (.x (Transformation|GetWorldLocation (Variables|Default|GetBox))))
      (Variables|Default|SetHas%20been%20tripped? true)
      (CallFunction|FireSound)
      (if (== (Variables|Default|GetText%20to%20fire) 6)
        (bind _asbp_player (Utilities|Casting|CastToBP_Player (Variables|Default|Getbp%20player)))
        (Variables|/Game/Blueprint/Character/Player/BP_Player.BP_Player_C|SetisHopeless _asbp_player true)
        (Audio|PlaySound2D "/Game/Sounds/Cinematic_boom.Cinematic_boom" 0.5 1.0 0.0 0 0)
        (Utilities|FlowControl|Delay 1.0)
        (bind _asbp_beam_end (Utilities|Casting|CastTobp_Beam_End (Variables|Default|Getlight%20beam)))
        (Transformation|SetWorldLocation _world (Math|Vector|MakeVector (.x (Transformation|GetWorldLocation (Variables|/Script/Engine.Character|GetCapsuleComponent (Variables|Default|Getbp%20player)))) (.y _returnvalue) (.z _returnvalue)) false false)
        (Variables|/Game/Blueprint/Eviros/bp_Beam_End.bp_Beam_End_C|SetEnd%20game _asbp_beam_end true)
        (Utilities|FlowControl|Delay 1.0)
        (Audio|PlaySound2D "/Game/Sounds/lostsoul.lostsoul" 1.0 1.0 0.0 0 0)
        (bind _asbp_text_manger (Utilities|Casting|CastToBP_TextManger (Variables|Default|Getclassref))
          (:then
            (Default|TextFires _asbp_text_manger (Variables|Default|GetText%20to%20fire))
            (Utilities|FlowControl|Delay 2.0)
            (Game|OpenLevel(byName) "NewMap"))
          (:CastFailed
            (Development|PrintString "FUCK")))
        (else
          (bind _asbp_text_manger_2 (Utilities|Casting|CastToBP_TextManger (Variables|Default|Getclassref))
            (:then
              (Default|TextFires _asbp_text_manger_2 (Variables|Default|GetText%20to%20fire))
              (Actor|DestroyActor))
            (:CastFailed
              (Development|PrintString "FUCK"))))))))

(fn ConstructionScript)